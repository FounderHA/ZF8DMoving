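; Bronze ingot resource pickup that the player can interact with in the world to collect.
; On interact, it passes the instigating controller's pawn to ServerRequestPickup, which requests the pickup from the server.
; Interaction getters supply the prompt and indicator widget classes, their screen offsets and the list of available interaction actions.
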(event EventOnInteract
  (params (InstigatorController :type Player%20Controller%20Object%20Reference) (InteractionID :type Name :default "None"))
  (Class|ZfItemPickup|ServerRequestPickup (Pawn|GetControlledPawn InstigatorController)))

(fn ConstructionScript)

(fn GetInteractionWidgetClass
  (return "/Game/Widgets/Interaction/WBP_Interaction.WBP_Interaction_C"))

(fn GetInteractionDataArray
  (return (Variables|Default|GetInteractionActions)))

(fn GetIndicatorWidgetClass
  (return "/Game/Widgets/Interaction/WBP_Indicator.WBP_Indicator_C"))

(fn GetInteractionWidgetOffset
  (return "(X=0.000000,Y=-25.000000)"))

(fn GetIndicatorWidgetOffset
  (return ""))