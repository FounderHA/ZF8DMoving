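; BP_Ore is an interactable ore node that players gather from.
; On interact, it sends a Gathering.Activate gameplay event to the instigator's pawn, passing itself as the optional object.
; Its ZfGatherableComponent reports depletion and respawn, which only print debug strings here; the HP-change handler is empty.
; Getter functions supply the interaction actions plus the indicator and interaction widget classes and their offsets.
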(event OnResourceRespawned(ZfGatherableComponent)
  (Development|PrintString "Respawn"))

(event OnResourceDepleted(ZfGatherableComponent)
  (Development|PrintString "Acabou"))

(event OnResourceHPChanged(ZfGatherableComponent)
  (params (CurrentHP :type Float%20%28single-precision%29) (MaxHP :type Float%20%28single-precision%29)))

(event EventOnInteract
  (params (InstigatorController :type Player%20Controller%20Object%20Reference) (InteractionID :type Name :default "None"))
  (Ability|SendGameplayEventtoActor (Pawn|GetControlledPawn InstigatorController) "(TagName=\"Gathering.Activate\")" (Utilities|Struct|MakeGameplayEventData "(TagName=\"Gathering.Activate\")" 0 0 self)))

(event EventBeginPlay)

(event EventOnPlayerEnterRange
  (params (InstigatorController :type Player%20Controller%20Object%20Reference)))

(fn ConstructionScript)

(fn GetIndicatorWidgetClass
  (return "/Game/Widgets/InteractionSystem/WBP_Indicator.WBP_Indicator_C"))

(fn GetIndicatorWidgetOffset
  (return "(X=0.000000,Y=-50.000000)"))

(fn GetInteractionDataArray
  (return (Variables|Default|GetInteractionActions)))

(fn GetInteractionWidgetClass
  (return "/Game/Widgets/InteractionSystem/WBP_Interaction.WBP_Interaction_C"))

(fn GetInteractionWidgetOffset
  (return "(X=0.000000,Y=-75.000000)"))