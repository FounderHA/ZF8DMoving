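; BP_ItemDropper is an actor that generates a randomized item and spawns it as a pickup at its own location.
; DropItem reads rarity probabilities from the item definition's rarity fragment, then feeds them to GenerateItem with tier and quality weights, level bonuses and tag bonuses.
; It synchronously loads the generated item's pickup class, spawns that actor and initializes it with the item.
; A missing rarity fragment stops the drop.
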(event EventDropItem
  (bind _asfragment__itemrarity (Utilities|Casting|CastToZfFragment_ItemRarity (Class|ZfItemDefinition|FindFragmentbyClass (Variables|Default|GetInItemDefinition) "/Script/ZF8DMoving.ZfFragment_ItemRarity")))
  (bind _returnvalue (Class|ZfItemGeneratorLibrary|GenerateItem self (Variables|Default|GetInItemDefinition) (Variables|/Script/ZF8DMoving.ZfFragment_ItemRarity|GetRarityProbability _asfragment__itemrarity) (Variables|Default|GetTierWeights) (Variables|Default|GetQualityWeights) 0 (Variables|Default|GetLevelBonuses) (Variables|Default|GetActiveTags) (Variables|Default|GetTagBonuses)))
  (bind _returnvalue_2 (Utilities|LoadClassAssetBlocking (Variables|/Script/ZF8DMoving.ZfItemDefinition|GetItemPickupActorClass (Variables|/Script/ZF8DMoving.ZfItemInstance|GetItemDefinition _returnvalue))))
  (bind _aszf_item_pickup (Utilities|Casting|CastToZfItemPickupClass _returnvalue_2))
  (bind _returnvalue_3 (Game|SpawnActorfromClass _aszf_item_pickup (Math|Transform|MakeTransform (Transformation|GetActorLocation) "0, 0, 0" "1.000000,1.000000,1.000000") "Undefined" "MultiplyWithRoot" 0 0))
  (Class|ZfItemPickup|InitializePickup _returnvalue_3 _returnvalue))

(fn ConstructionScript)