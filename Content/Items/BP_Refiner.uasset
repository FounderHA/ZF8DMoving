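; BP_Refiner is an interactable refinery actor whose behavior centers on its RefineryComponent.
; Local interaction creates a WBP_RefineryMenu bound to that component and adds it to the instigating player's viewport.
; Getter functions supply the indicator and interaction prompt widgets, their offsets and the action data.
; Tick loops over the input slots and, on authority only, prints each item's name and stack count on screen as debug output.
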(event EventTick
  (params (DeltaSeconds :type Float%20%28single-precision%29))
  (bind _refinerycomponent (Variables|Default|GetRefineryComponent))
  (for _index (range 0 (- (Variables|/Script/ZF8DMoving.ZfRefineryData|GetInputSlotCapacity (Variables|/Script/ZF8DMoving.ZfRefineryComponent|GetRefineryData (Variables|Default|GetRefineryComponent))) 1))
    (Utilities|IsValid (Class|ZfRefineryComponent|GetSlotItem _refinerycomponent (Class|ZfRefineryComponent|GetInputSlots _refinerycomponent) _index)
      (:Is%20Valid
        (Networking|SwitchHasAuthority
          (:Authority
            (Development|PrintString (Utilities|String|ToString(Text) (Utilities|Text|FormatText "{A}: {B}" (Utilities|String|ToString(Text) (Class|ZfItemInstance|GetItemName (Class|ZfRefineryComponent|GetSlotItem _refinerycomponent (Class|ZfRefineryComponent|GetInputSlots _refinerycomponent) _index))) (Class|ZfItemInstance|GetCurrentStack (Class|ZfRefineryComponent|GetSlotItem _refinerycomponent (Class|ZfRefineryComponent|GetInputSlots _refinerycomponent) _index)))) true false "(R=0.328125,G=0.126963,B=0.000000,A=1.000000)" 0.0)))))))

(event EventOnInteractLocal
  (params (InstigatorPC :type Player%20Controller%20Object%20Reference) (InteractionID :type Name :default "None"))
  (bind _returnvalue (UserInterface|CreateWidget "/Game/Widgets/Refinery/WBP_RefineryMenu.WBP_RefineryMenu_C" InstigatorPC (Variables|Default|GetRefineryComponent)))
  (bind _output_get (Variables|Default|SetWBP_RefineryMenu _returnvalue))
  (UserInterface|Viewport|AddtoViewport _output_get 0))

(fn ConstructionScript)

(fn GetIndicatorWidgetClass
  (return "/Game/Widgets/Interaction/WBP_Indicator.WBP_Indicator_C"))

(fn GetIndicatorWidgetOffset
  (return "(X=0.000000,Y=-100.000000)"))

(fn GetInteractionDataArray
  (return (Variables|Default|GetActionKeys)))

(fn GetInteractionWidgetClass
  (return "/Game/Widgets/Interaction/WBP_Interaction.WBP_Interaction_C"))

(fn GetInteractionWidgetOffset
  (return "(X=0.000000,Y=-125.000000)"))