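; Sword pickup actor Blueprint that shows the current stack count of its item instance on a text render.
; On BeginPlay, if the item instance is missing, the authority initializes the pickup from a variable, while remote clients take a short delay branch.
; The text is then set from the instance's stack value.
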(event EventBeginPlay
  (Utilities|IsValid (Variables|Default|GetItemInstance)
    (:Is%20Valid
      _)
    (:Is%20Not%20Valid
      (Networking|SwitchHasAuthority
        (:Authority
          (Class|ZfItemPickup|InitializePickup (Variables|Default|GetNewVar)))
        (:Remote
          (Utilities|FlowControl|Delay 0.2)))))
  (Rendering|Components|TextRender|SetText (Variables|Default|GetTextRender) (Utilities|Text|ToText(Integer) (Class|ZfItemInstance|GetCurrentStack (Variables|Default|GetItemInstance)))))

(fn ConstructionScript)