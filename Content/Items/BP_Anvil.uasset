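; BP_Anvil is an interactable anvil item that opens a crafting menu for the player who uses it.
; OnInteractLocal creates WBP_CraftMenu for the instigating player controller, passes the anvil as TargetActor and adds it to the viewport, while OnInteract stays empty.
; Getter functions supply the indicator and interaction widget classes, their screen offsets and the ActionKeys array as interaction data.
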(event EventOnInteractLocal
  (params (InstigatorPC :type Player%20Controller%20Object%20Reference) (InteractionID :type Name :default "None"))
  (bind _returnvalue (UserInterface|CreateWidget "/Game/Widgets/Crafting/WBP_CraftMenu.WBP_CraftMenu_C" InstigatorPC self))
  (bind _output_get (Variables|Default|SetWBP_CraftMenu _returnvalue))
  (UserInterface|Viewport|AddtoViewport _output_get 0))

(event EventOnInteract
  (params (InstigatorController :type Player%20Controller%20Object%20Reference) (InteractionID :type Name :default "None")))

(fn ConstructionScript)

(fn GetIndicatorWidgetClass
  (return "/Game/Widgets/Interaction/WBP_Indicator.WBP_Indicator_C"))

(fn GetIndicatorWidgetOffset
  (return "(X=0.000000,Y=-100.000000)"))

(fn GetInteractionDataArray
  (return (Variables|Default|GetActionKeys)))

(fn GetInteractionWidgetClass
  (return "/Game/Widgets/Interaction/WBP_Interaction.WBP_Interaction_C"))

(fn GetInteractionWidgetOffset
  (return "(X=0.000000,Y=-125.000000)"))