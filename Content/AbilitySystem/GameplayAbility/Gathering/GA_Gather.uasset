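; GA_Gather is a gathering gameplay ability that handles the skill-check UI shown while harvesting a resource.
; When a client round begins, it creates skill-check and resource-HP widgets for the target gatherable, unless a skill check already exists.
; Drop resolution or cancellation removes both widgets, with HP widget cleanup nested under the skill-check validity check.
; QTE start is empty, and hit impact only prints debug text.
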(event EventOnClientRoundBegun
  (params (GoodSize :type Float%20%28single-precision%29) (PerfectSize :type Float%20%28single-precision%29) (NeedleRotTime :type Float%20%28single-precision%29))
  (Utilities|IsValid (Variables|Default|GetWBP_SkillCheck)
    (:Is%20Not%20Valid
      (Utilities|FlowControl|Sequence
        (:then_0
          (bind _returnvalue (UserInterface|CreateWidget "/Game/Widgets/WBP_SkillCheck.WBP_SkillCheck_C"))
          (bind _output_get (Variables|Default|SetWBP_SkillCheck _returnvalue))
          (UserInterface|Viewport|AddtoViewport _output_get 0)
          (Class|ZfGatheringSkillCheckWidget|InitSkillCheck (Variables|Default|GetWBP_SkillCheck) (Class|ZfGAGatheringBase|GetTargetGatherableComponent)))
        (:then_1
          (bind _returnvalue_2 (UserInterface|CreateWidget "/Game/Widgets/Gathering/WBP_ResourceHP.WBP_ResourceHP_C" 0 0))
          (Class|ZfResourceHPWidget|InitResourceWidget _returnvalue_2 (Components|GetOwner (Class|ZfGAGatheringBase|GetTargetGatherableComponent)))
          (Class|UserWidget|SetAlignmentinViewport _returnvalue_2 "(X=1.000000,Y=1.000000)")
          (UserInterface|Viewport|AddtoViewport _returnvalue_2 0)
          (Variables|Default|SetWBP_ResourceHP _returnvalue_2))))))

(event EventOnQTEStarted
  (params (GoodSize :type Float%20%28single-precision%29) (PerfectSize :type Float%20%28single-precision%29) (NeedleRotationTime :type Float%20%28single-precision%29)))

(event EventOnHitImpact
  (params (HitResult :type EZfGatherHitResult%20Enum :default "Perfect") (DamageDealt :type Float%20%28single-precision%29) (RemainingHP :type Float%20%28single-precision%29))
  (Development|PrintString "Impacto")
  (Utilities|IsValid (Variables|Default|GetWBP_SkillCheck)))

(event EventOnDropsResolved
  (params (Drops :type Array%20of%20Zf%20Gather%20Drop%20Result%20Structures) (ScoreFinal :type Float%20%28single-precision%29))
  (Development|PrintString "Drop")
  (Utilities|IsValid (Variables|Default|GetWBP_SkillCheck)
    (:Is%20Valid
      (Widget|RemovefromParent (Variables|Default|GetWBP_SkillCheck))
      (Variables|Default|SetWBP_SkillCheck 0)
      (Utilities|IsValid (Variables|Default|GetWBP_ResourceHP)
        (:Is%20Valid
          (Widget|RemovefromParent (Variables|Default|GetWBP_ResourceHP))
          (Variables|Default|SetWBP_ResourceHP 0))))))

(event EventOnGatherCancelled
  (Development|PrintString "cancelled")
  (Utilities|IsValid (Variables|Default|GetWBP_SkillCheck)
    (:Is%20Valid
      (Widget|RemovefromParent (Variables|Default|GetWBP_SkillCheck))
      (Variables|Default|SetWBP_SkillCheck 0)
      (Utilities|IsValid (Variables|Default|GetWBP_ResourceHP)
        (:Is%20Valid
          (Widget|RemovefromParent (Variables|Default|GetWBP_ResourceHP))
          (Variables|Default|SetWBP_ResourceHP 0))))))