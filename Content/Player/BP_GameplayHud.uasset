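; BP_GameplayHud is a player HUD Blueprint that opens and closes the character menu through its ToggleInventory event.
; Opening creates WBP_CharacterMenu, stores it in MainHud, switches input to game and UI with focus on the menu, and shows the cursor.
; Closing removes the widget, restores game-only input, hides the cursor and clears MainHud.
; Creation of WBP_GameplayHud is present but unconnected, and BeginPlay is empty.
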(event Custom|ToggleInventory
  (bind _returnvalue (Game|Player|GetOwningPlayerController))
  (bind _returnvalue_2 (Game|Player|GetOwningPlayerController))
  (bind _mainhud (Variables|Default|GetMainHud)
    (:then
      (Widget|RemovefromParent _mainhud)
      (Input|SetInputModeGameOnly _returnvalue_2 false)
      (Variables|/Script/Engine.PlayerController|SetbShowMouseCursor _returnvalue_2 false)
      (Variables|Default|SetMainHud 0))
    (:else
      (bind _returnvalue_3 (UserInterface|CreateWidget "/Game/Widgets/WBP_CharacterMenu.WBP_CharacterMenu_C"))
      (bind _output_get (Variables|Default|SetMainHud _returnvalue_3))
      (UserInterface|Viewport|AddtoViewport _output_get 0)
      (Input|SetInputModeGameandUI _returnvalue _output_get "DoNotLock" true false)
      (Variables|/Script/Engine.PlayerController|SetbShowMouseCursor _returnvalue true))))

(event EventBeginPlay)

(fn ConstructionScript)