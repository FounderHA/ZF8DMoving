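; Player State Blueprint that carries the player's Ability System, Inventory and Equipment components.
; On BeginPlay it grants the Gather and Use Item gameplay abilities to the Ability System Component, with no authority check in the graph.
; Disconnected leftovers hold level-up and XP ability grants, a gameplay effect application, and debug printouts of inventory items, equipment tags and an attribute value.
; Tick and ApplyRecalculateAttribute are empty.
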(event EventBeginPlay
  (GameplayAbilities|GiveAbility (Variables|Default|GetAbilitySystemComponent) "/Game/AbilitySystem/GameplayAbility/Gathering/GA_Gather.GA_Gather_C" 0 -1)
  (GameplayAbilities|GiveAbility (Variables|Default|GetAbilitySystemComponent) "/Game/AbilitySystem/GameplayAbility/Misc/GA_UseItem.GA_UseItem_C" 0 -1))

(event EventApplyRecalculateAttribute
  (params (InAttributeType :type Byte :default 0)))

(event EventTick
  (params (DeltaSeconds :type Float%20%28single-precision%29)))

(fn ConstructionScript)