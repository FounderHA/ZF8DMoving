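; Player HUD that puts the gameplay HUD widget on screen at BeginPlay and toggles the character menu through ToggleInventory.
; The toggle creates or removes the menu widget, switching input mode and mouse cursor to match.
; A similar toggle for the Novice skill tree region widget, which passes in the owning pawn's PlayerState, is present but unconnected and never runs.
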(event Custom|ToggleInventory
  (bind _returnvalue (Game|Player|GetOwningPlayerController))
  (bind _returnvalue_2 (Game|Player|GetOwningPlayerController))
  (bind _wbp_charactermenu (Variables|Default|GetWBP_CharacterMenu)
    (:then
      (Widget|RemovefromParent _wbp_charactermenu)
      (Input|SetInputModeGameOnly _returnvalue_2 false)
      (Variables|/Script/Engine.PlayerController|SetbShowMouseCursor _returnvalue_2 false)
      (Variables|Default|SetWBP_CharacterMenu 0))
    (:else
      (bind _returnvalue_3 (UserInterface|CreateWidget "/Game/Widgets/WBP_CharacterMenu.WBP_CharacterMenu_C"))
      (bind _output_get (Variables|Default|SetWBP_CharacterMenu _returnvalue_3))
      (UserInterface|Viewport|AddtoViewport _output_get 0)
      (Input|SetInputModeGameandUI _returnvalue _output_get "DoNotLock" true false)
      (Variables|/Script/Engine.PlayerController|SetbShowMouseCursor _returnvalue true))))

(event EventBeginPlay
  (bind _returnvalue (UserInterface|CreateWidget "/Game/Widgets/WBP_GameplayHud.WBP_GameplayHud_C"))
  (UserInterface|Viewport|AddtoViewport _returnvalue 0))

(fn ConstructionScript)